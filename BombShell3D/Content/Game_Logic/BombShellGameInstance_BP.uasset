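; Game instance Blueprint that hands Steam friend list results to a 3D selection UI in the world.
; When the friend request completes, it finds all TestActor instances and checks their widget components for the ThreeD tag.
; For each match, it casts the user widget to Selection_UI_3D, forwards the friends list to it and prints debug messages.
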(event EventOnGetSteamFriendRequestCompleteUMG
  (params (BPFriendsLists :type Array%20of%20Steam%20Friend%20Info%20Structures))
  (bind _outactors (Actor|GetAllActorsOfClass "/Game/Display/UI/TestActor.TestActor_C"))
  (for _array_element _outactors
    (if (Components|ComponentHasTag (Variables|/Game/Display/UI/TestActor.TestActor_C|GetWidget _array_element) "ThreeD")
      (bind _asselection_ui_3d (Utilities|Casting|CastToSelection_UI_3D (UserInterface|GetUserWidgetObject (Variables|/Game/Display/UI/TestActor.TestActor_C|GetWidget _array_element))))
      (Utilities|IsValid _asselection_ui_3d
        (:Is%20Valid
          (Default|GetSteamFriendRequestCompleted _asselection_ui_3d BPFriendsLists)
          (Development|PrintString "Game Instance reached"))
        (:Is%20Not%20Valid
          (Development|PrintString "NOT VALID, PROBLEM"))))))