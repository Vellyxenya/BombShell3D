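; Bomb actor that aligns itself to a grid when play begins.
; BeginPlay passes its location through SnapLocation and teleports the actor to the result without sweeping.
; SnapLocation snaps each axis to GridSize, then lowers Z by a fixed offset.
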(event EventBeginPlay
  (bind _finallocation (CallFunction|SnapLocation (Transformation|GetActorLocation)))
  (Transformation|SetActorLocation _finallocation false true))

(fn ConstructionScript)

(fn SnapLocation
  (params (InVec :type Vector))
  (bind (_x _y _z) (Math|Vector|BreakVector InVec))
  (bind _gridsize (Variables|Default|GetgridSize))
  (return (Math|Vector|MakeVector (Math|Float|SnapToGrid(Float) _x _gridsize) (Math|Float|SnapToGrid(Float) _y _gridsize) (- (Math|Float|SnapToGrid(Float) _z _gridsize) 1e+02))))